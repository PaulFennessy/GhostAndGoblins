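; Procedurall_BP is an actor that lays out a flat grid of instanced static meshes.
; Its construction script runs nested loops over NumberX and NumberY, adding an instance at each cell with fixed 500-unit spacing in local space.
; The event graph holds only disabled default events, so all work happens at construction.
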(event EventBeginPlay)

(event Collision|EventActorBeginOverlap
  (params (OtherActor :type Actor%20Object%20Reference)))

(event EventTick
  (params (DeltaSeconds :type Float%20%28single-precision%29)))

(fn ConstructionScript
  (for _index (range 0 (- (Variables|Default|GetNumberX) 1))
    (LocalVariables|SetSetX _index)
    (for _index_2 (range 0 (- (Variables|Default|GetNumberY) 1))
      (LocalVariables|SetSetY _index_2)
      (Components|InstancedStaticMesh|AddInstance (Variables|Default|GetInstancedStaticMesh) (Math|Transform|MakeTransform (Math|Vector|MakeVector (* (LocalVariables|GetSetX) 5e+02) (* (LocalVariables|GetSetY) 5e+02) 0.0)) false))))